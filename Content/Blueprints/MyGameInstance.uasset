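; Game instance that builds hard-coded 2D layouts of square rooms as RenderingInformation segments when the game initializes.
; Init fills three arrays (Segments, SegmentsII, SegmentsIII), each outlining a room with a centered opening on one side.
; Only Segments stores its opening as a non-wall segment; the matching nodes for the other two are disconnected, leaving gaps.
; The first two rooms share the opening edge, while the third overlaps both.
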(event `self.ReceiveInit`
  (`KismetArrayLibrary.Array_Add` (`self.Segments`) (make `RenderingInformation` (500.0 -50.0) (500.0 -500.0)))
  (`KismetArrayLibrary.Array_Add` (`self.Segments`) (make `RenderingInformation` (500.0 -50.0) (500.0 50.0) "PLUS_X" false))
  (`KismetArrayLibrary.Array_Add` (`self.Segments`) (make `RenderingInformation` (500.0 50.0) (500.0 500.0)))
  (`KismetArrayLibrary.Array_Add` (`self.Segments`) (make `RenderingInformation` (500.0 500.0) (-500.0 500.0)))
  (`KismetArrayLibrary.Array_Add` (`self.Segments`) (make `RenderingInformation` (500.0 -500.0) (-500.0 -500.0)))
  (`KismetArrayLibrary.Array_Add` (`self.Segments`) (make `RenderingInformation` (-500.0 500.0) (-500.0 -500.0)))
  (`KismetArrayLibrary.Array_Add` (`self.SegmentsII`) (make `RenderingInformation` (500.0 -50.0) (500.0 -500.0)))
  (`KismetArrayLibrary.Array_Add` (`self.SegmentsII`) (make `RenderingInformation` (500.0 50.0) (500.0 500.0)))
  (`KismetArrayLibrary.Array_Add` (`self.SegmentsII`) (make `RenderingInformation` (1500.0 500.0) (500.0 500.0)))
  (`KismetArrayLibrary.Array_Add` (`self.SegmentsII`) (make `RenderingInformation` (1500.0 -500.0) (500.0 -500.0)))
  (`KismetArrayLibrary.Array_Add` (`self.SegmentsII`) (make `RenderingInformation` (1500.0 500.0) (1500.0 -500.0)))
  (`KismetArrayLibrary.Array_Add` (`self.SegmentsIII`) (make `RenderingInformation` (0.0 -500.0) (0.0 -50.0)))
  (`KismetArrayLibrary.Array_Add` (`self.SegmentsIII`) (make `RenderingInformation` (0.0 50.0) (0.0 500.0)))
  (`KismetArrayLibrary.Array_Add` (`self.SegmentsIII`) (make `RenderingInformation` (1000.0 500.0) (0.0 500.0)))
  (`KismetArrayLibrary.Array_Add` (`self.SegmentsIII`) (make `RenderingInformation` (1000.0 -500.0) (-0.0 -500.0)))
  (`KismetArrayLibrary.Array_Add` (`self.SegmentsIII`) (make `RenderingInformation` (1000.0 500.0) (1000.0 -500.0))))
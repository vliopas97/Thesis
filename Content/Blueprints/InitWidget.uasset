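; InitWidget is an actor that shows a start-prompt loading screen through a stereo layer, apparently for VR.
; On BeginPlay it sets the LoadingScreenWidget message to prompt a right trigger press.
; Tick waits for the widget component's render target to become valid, then assigns it once as the stereo layer texture.
; A Hide event turns off visibility on both the widget and the stereo layer.
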(event `self.ReceiveBeginPlay`
  (bind _asloading_screen_widget (cast `/Game/Widgets/LoadingScreenWidget` (`WidgetComponent.GetUserWidgetObject` (`self.Widget`))))
  (set `LoadingWidgetTemplate.Message` "Press Right Trigger to Start" _asloading_screen_widget))

(event `self.ReceiveTick`
  (params (DeltaSeconds :type "Float (single-precision)"))
  (bind _returnvalue (`WidgetComponent.GetRenderTarget` (`self.Widget`)))
  (`/Engine/EditorBlueprintResources/StandardMacros.IsValid` _returnvalue
    (:`Is Valid`
      (`/Engine/EditorBlueprintResources/StandardMacros.DoOnce` false
        (:`Completed`
          (`StereoLayerComponent.SetTexture` (`self.StereoLayer`) _returnvalue))))))

(event `Hide`
  (`SceneComponent.SetVisibility` (`self.Widget`) false false)
  (`SceneComponent.SetVisibility` (`self.StereoLayer`) false false))

(event `self.ReceiveDestroyed`)

(event `self.ReceiveEndPlay`
  (params (EndPlayReason :type "EEndPlayReason Enum" :default "Destroyed")))

(fn `UserConstructionScript`)
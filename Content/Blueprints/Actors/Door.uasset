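; Interactive door actor that swings away from the player and streams rooms in and out through the game instance.
; Entering its collision box prepares room data and shows a side-aware 3D prompt; a camera line trace on Interact renders the room and plays the swing timeline.
; Leaving reverses the swing, then player-side checks decide whether to clear the previous room or discard the new one.
; The construction script fits the overhead wall to room height.
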(event `self.ReceiveBeginPlay`
  (`|CreateWidget` "/Game/Widgets/3DInteract_Prompt_Door.3DInteract_Prompt_Door_C")
  (set `self.InteractWidget` null)
  (`self.EnableInput` (`GameplayStatics.GetPlayerController` 0))
  (bind _direction_copy (`self.DeterminePlayerDirection`)
    (:`Out`
      (set `self.PlayerPositionToDoor` _direction_copy))))

(event `InputAction|Interact` :consume false
  (params (Key :type "Key Structure"))
  ;[1 1 1] Door Interact Key
  (:`Pressed`
    (bind _aszedplayer (cast `/Game/Blueprints/ZEDPlayer` (`GameplayStatics.GetPlayerPawn` 0)))
    (bind _camera (`VRPawn.Camera` _aszedplayer))
    (bind _returnvalue (`SceneComponent.K2_GetComponentLocation` _camera))
    (bind (_hitlocation _hitnormal _bonename _outhit _returnvalue_2) (`PrimitiveComponent.K2_LineTraceComponent` (`self.Door`) _returnvalue (+ _returnvalue (* (`KismetMathLibrary.GetForwardVector` (`SceneComponent.K2_GetComponentRotation` _camera)) 150.0)) false true false))
    (bind _returnvalue_3 (`self.GetEnableInteraction`))
    (if (and _returnvalue_2 _returnvalue_3)
      (if (not (`self.Locked`))
        (`SceneComponent.SetVisibility` (`self.Widget`) false false)
        (if (not (`self.Opened`))
          (`self.Load New Room`)
          ;[1 1 1] Open and Close the Door
          (`/Engine/EditorBlueprintResources/StandardMacros.Gate` true :!label _label
            (:`Exit`
              (bind _direction_copy (`self.DeterminePlayerDirection`)
                (:`Out`
                  (bind _output_get (set `self.DirectionChange` _direction_copy))
                  (bind (_direction _open_close) (`Timeline|DoorOpen` :!label _label_2)
                    (:`Update`
                      (`SceneComponent.K2_SetRelativeRotation` (`self.Door`) (`KismetMathLibrary.MakeRotator` 0.0 0.0 (+ (* (`KismetMathLibrary.Lerp` (`self.CloseAngle`) (`self.OpenAngle`) _open_close) (`KismetMathLibrary.SelectFloat` -1.0 1.0 (`self.DirectionChange`))) 90.0)) false false))
                    (:`Finished`
                      ;[1 1 1] When Door Closes Destroy Previous Room
                      (if (`self.Opened`)
                        (bind _direction_copy_2 (`self.DeterminePlayerDirection`)
                          (:`Out`
                            (if (!= _direction_copy_2 _output_get)
                              (`self.Clear Previous Room`)
                              (`self.SwapDoorDirection`)
                              (else
                                (`self.Delete New Room`
                                  (:`Out`
                                    _))))
                            (set `self.Opened` false)))))))))))))))

(event `self.CollisionBox.OnComponentBeginOverlap`
  (params (OverlappedComponent :type "PrimitiveComponent Object Reference") (OtherActor :type "Actor Object Reference") (OtherComp :type "PrimitiveComponent Object Reference") (OtherBodyIndex :type Integer) (bFromSweep :type Boolean) (SweepResult :type "HitResult Structure (by ref)"))
  ;[1 1 1] Character approaches Door, begins overlap with CollisionBox
  (cast `/Game/Blueprints/ZEDPlayer` OtherActor)
  (bind _direction_copy (`self.DeterminePlayerDirection`)
    (:`Out`
      (set `self.PlayerPositionToDoor` _direction_copy)
      (set `self.CharacterWithinRange` true)
      (bind _returnvalue (`self.GetLoadNewRoom`))
      (if _returnvalue
        (bind _asmy_game_instance_code (cast `MyGameInstanceCode` (`GameplayStatics.GetGameInstance`)))
        (`MyGameInstanceCode.GetRoomInformation` _asmy_game_instance_code self)
        (`MyGameInstanceCode.AttachDoor` _asmy_game_instance_code self)
        (`self.SetLoadNewRoom` false))
      (bind _returnvalue_2 (`self.GetEnableInteraction` :!label _label_3))
      (if (or (`self.Opened`) (not _returnvalue_2))
        (`KismetSystemLibrary.Delay` 0.1)
        (if (`PrimitiveComponent.IsOverlappingActor` (`self.CollisionBox`) (`GameplayStatics.GetPlayerPawn` 0))
          (goto _label_3))
        (else
          (`self.Spawn 3D Widget`
            (:`Out`
              ;;[1 0.9277 0.2728] If Door is Locked then block opening and notify player
              (if (`self.Locked`)
                (bind _as3dinteract_prompt_door (cast `/Game/Widgets/3DInteract_Prompt_Door` (`WidgetComponent.GetUserWidgetObject` (`self.Widget`))))
                (set `/Game/Widgets/3DInteract_Prompt_Door.Text` "Locked" _as3dinteract_prompt_door)
                (else
                  (goto _label :!via `Open`))))))))))

(event `self.CollisionBox.OnComponentEndOverlap`
  (params (OverlappedComponent :type "PrimitiveComponent Object Reference") (OtherActor :type "Actor Object Reference") (OtherComp :type "PrimitiveComponent Object Reference") (OtherBodyIndex :type Integer))
  ;[1 1 1] Actor leaves Door, ends overlap with CollisionBox
  (cast `/Game/Blueprints/ZEDPlayer` OtherActor)
  (set `self.CharacterWithinRange` false)
  (`self.SetEnableInteraction` false)
  (`self.Remove 3D Widget`
    (:`Out`
      (if (`KismetMathLibrary.NearlyEqual_FloatFloat` (.yaw (.rotation (`SceneComponent.GetRelativeTransform` (`self.Door`)))) 90.0 0.001)
        (`self.Delete New Room`
          (:`Out`
            (goto _label_2 :!via `Reverse`)))
        (else
          (set `self.Opened` true)
          (goto _label_2 :!via `Reverse`))))))

(event `self.Toggle.OnComponentEndOverlap`
  (params (OverlappedComponent :type "PrimitiveComponent Object Reference") (OtherActor :type "Actor Object Reference") (OtherComp :type "PrimitiveComponent Object Reference") (OtherBodyIndex :type Integer)))

(event `Load New Room`
  (if (not (`self.Locked`))
    (bind _asmy_game_instance (cast `/Game/Blueprints/MyGameInstance` (`GameplayStatics.GetGameInstance`)))
    (`MyGameInstanceCode.RenderRoom` _asmy_game_instance self)))

(event `Clear Previous Room`
  (bind _asmy_game_instance (cast `/Game/Blueprints/MyGameInstance` (`GameplayStatics.GetGameInstance`)))
  (`MyGameInstanceCode.ClearPreviousRoom` _asmy_game_instance self))

(fn `UserConstructionScript`
  (bind _asmy_game_instance (cast `/Game/Blueprints/MyGameInstance` (`GameplayStatics.GetGameInstance`)))
  (set `self.WallsHeight` (`MyGameInstanceCode.WallHeight` _asmy_game_instance))
  (`SceneComponent.SetWorldScale3D` (`self.Wall`) (`KismetMathLibrary.MakeVector` 0.25 1.28125 (/ (- (`self.WallsHeight`) 211.0) 100.0)))
  (`SceneComponent.K2_SetRelativeLocation` (`self.Wall`) (`KismetMathLibrary.MakeVector` 0.0 0.0 (+ (`self.DoorFrameTop`) (/ (- (`self.WallsHeight`) (`self.DoorFrameTop`)) 2.0))) false false))

(fn `VectorsAngle`
  (params (A :type "/Game/ThirdPersonBP/Blueprints/ThirdPersonCharacter Object Reference"))
  (returns (NewParam :type "Float (double-precision)"))
  (locals (NewLocalVar_0 :type "SpringArmComponent Object Reference"))
  (bind _returnvalue (`KismetMathLibrary.Normal` (`SceneComponent.GetForwardVector` (`Character.Mesh` A))))
  (bind _returnvalue_2 (`SceneComponent.GetForwardVector` (`self.DefaultSceneRoot`)))
  (return (`KismetMathLibrary.FMin` (`KismetMathLibrary.DegAcos` (`KismetMathLibrary.Dot_VectorVector` _returnvalue (`KismetMathLibrary.Normal` _returnvalue_2))) (`KismetMathLibrary.DegAcos` (`KismetMathLibrary.Dot_VectorVector` _returnvalue (`KismetMathLibrary.NegateVector` _returnvalue_2))))))
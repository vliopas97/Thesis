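; HumanAI is an AI-driven pawn that can be sent to a destination and spawns an effect when destroyed.
; The Moveto event runs AI Move To using the destination's X and Y while keeping the pawn's current height.
; On destruction, RenderEffects spawns the NSTest system at the actor's location.
; BeginPlay and Destroyed also print debug strings; overlap and Tick are unused.
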(event `self.ReceiveBeginPlay`
  (`KismetSystemLibrary.PrintString` "Hello"))

(event `self.ReceiveDestroyed`
  (`KismetSystemLibrary.PrintString` "bye")
  (`self.RenderEffects`))

(event `self.RenderEffects`
  (`NiagaraFunctionLibrary.SpawnSystemAtLocation` "/Game/Blueprints/NSTest.NSTest" (`self.K2_GetActorLocation`)))

(event `self.MoveTo`
  (params (Destination :type "Vector2D Structure (by ref)"))
  (bind (_returnvalue_x _returnvalue_y _returnvalue_z) (`KismetMathLibrary.BreakVector` (`self.K2_GetActorLocation` self)))
  (`|AIMoveTo` self (`KismetMathLibrary.MakeVector` Destination_X Destination_Y _returnvalue_z) null))

(fn `UserConstructionScript`)
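; Torch actor whose point light flickers during play.
; On BeginPlay it picks one of two intensity curves at random, so separate torches can flicker differently.
; A Flickering timeline then drives the PointLight intensity from the chosen curve, scaled by a fixed multiplier.
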(event `self.ReceiveBeginPlay`
  (set `self.IntensityPick` (`KismetMathLibrary.RandomBool`))
  (bind (_direction _intensity _intensity2) (`Timeline|Flickering`)
    (:`Update`
      (if (`self.IntensityPick`)
        (`LightComponent.SetIntensity` (`self.PointLight`) (* _intensity 5000.0))
        (else
          (`LightComponent.SetIntensity` (`self.PointLight`) (* _intensity2 5000.0)))))))

(fn `UserConstructionScript`)